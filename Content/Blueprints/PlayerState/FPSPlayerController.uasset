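; FPS player controller that can switch the controlled pawn's input on or off.
; SetPlayerEnablestate enables input on the pawn, or disables it and calls DisableFire when the pawn is an FPS_Character.
; BeginPlay and Tick are empty, and the nodes for caching the game state, disabling pawn 0's input and toggling the mouse cursor are disconnected.
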(event `self.ReceiveBeginPlay`)

(fn `SetPlayerEnablestate`
  (params (SetPlayerEnabled :type Boolean))
  (bind _returnvalue (`self.K2_GetPawn`))
  (if SetPlayerEnabled
    (`self.EnableInput` _returnvalue self)
    (else
      (`self.DisableInput` _returnvalue self)
      (bind _asfps_character (cast `/Game/Blueprints/Character/FPS_Character` _returnvalue))
      (`/Game/Blueprints/Character/FPS_Character.Disable Fire` _asfps_character))))

(fn `UserConstructionScript`)
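; FPS player state that puts up the game mode HUD and holds logic for enabling or disabling its player.
; BeginPlay adds a GameModeHUD widget to the viewport and caches the FPSGameState.
; SetPlayeStaterEnable forwards an enable flag to the pawn's FPSPlayerController.
; CheckEnableInputs allows pawn input only while the session is In Progress, but its call in the event graph is disconnected.
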(event `self.ReceiveBeginPlay`
  (`|ExecutionSequence`
    (:`then_0`
      (bind _returnvalue (`|CreateWidget` "/Game/Blueprints/UI/HUD/GameModeHUD.GameModeHUD_C"))
      (bind _output_get (set `self.GM_HUD` _returnvalue))
      (`UserWidget.AddToViewport` _output_get 0))
    (:`then_1`
      (bind _asfpsgame_state (cast `/Game/Blueprints/GameModes/FPSGameState` (`GameplayStatics.GetGameState`)))
      (bind _output_get_2 (set `self.GameSate` _asfpsgame_state)))))

(fn `CheckEnableInputs`
  (bind _pawnprivate (`self.PawnPrivate`))
  (bind _gamesate (`self.GameSate`))
  (bind _pawnprivate_2 (`self.PawnPrivate`))
  (`/Engine/EditorBlueprintResources/StandardMacros.IsValid` (`self.PawnPrivate`)
    (:`Is Valid`
      (`/Engine/EditorBlueprintResources/StandardMacros.IsValid` _gamesate
        (:`Is Valid`
          (switch `/Game/Blueprints/GameModes/SessionState_E` (`/Game/Blueprints/GameModes/FPSGameState.getSessionState` _gamesate)
            (:`NewEnumerator0`
              (bind _asplayer_controller (cast `PlayerController` (`Pawn.GetController` _pawnprivate) :!label _label))
              (`self.DisableInput` _pawnprivate _asplayer_controller))
            (:`NewEnumerator1`
              (bind _asplayer_controller_2 (cast `PlayerController` (`Pawn.GetController` _pawnprivate_2)))
              (`self.EnableInput` _pawnprivate_2 _asplayer_controller_2))
            (:`NewEnumerator2`
              (goto _label))
            (:`NewEnumerator3`
              (goto _label))
            (:`NewEnumerator4`
              (goto _label))))))))

(fn `SetPlayeStaterEnable`
  (params (SetPlayerEnabled :type Boolean))
  (bind _pawnprivate (`self.PawnPrivate`))
  (`/Engine/EditorBlueprintResources/StandardMacros.IsValid` _pawnprivate
    (:`Is Valid`
      (bind _asfpsplayer_controller (cast `/Game/Blueprints/PlayerState/FPSPlayerController` (`Pawn.GetController` _pawnprivate)))
      (`/Game/Blueprints/PlayerState/FPSPlayerController.SetPlayerEnablestate` _asfpsplayer_controller SetPlayerEnabled))))

(fn `UserConstructionScript`)
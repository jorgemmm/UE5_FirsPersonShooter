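; Actor component that tracks an owner's health and death state.
; UpdateHealth reduces incoming damage by Constitution while keeping at least 1 point of loss, then clamps Health between zero and the default attribute value.
; It then recalculates IsDeath from Health, which getters expose along with current and default health.
; BeginPlay and Tick are empty, and a debug print is disconnected.
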(event `self.ReceiveBeginPlay`)

(fn `CalculeDead`
  (if (<= (`self.Health`) 0.0)
    (set `self.bIsDeath` true)
    (else
      (set `self.bIsDeath` false))))

(fn `CheckIsDead`
  (returns (bIsDeath :type Boolean))
  (return (`self.bIsDeath`)))

(fn `GetHealth`
  (returns (Health :type "Float (double-precision)"))
  (return (`self.Health`)))

(fn `getvalueDefault`
  (returns (ValueAtributteDefault :type "Float (double-precision)"))
  (return (`self.ValueAtributteDefault`)))

(fn `UpdateHealth`
  (params (ChangeHealth :type "Float (double-precision)"))
  (locals (ChangeValue :type "Float (double-precision)"))
  (bind _changevalue (`local.ChangeValue`))
  (bind _output_get (set `local.ChangeValue` ChangeHealth))
  (if (< _output_get 0.0)
    (set `local.ChangeValue` (`KismetMathLibrary.FClamp` (+ _changevalue (`self.Constitution`)) _changevalue -1.0)))
  (bind _output_get_2 (set `self.Health` (`KismetMathLibrary.FClamp` (+ (`local.ChangeValue`) (`self.Health`)) 0.0 (`self.ValueAtributteDefault`))))
  (`self.CalculeDead`))
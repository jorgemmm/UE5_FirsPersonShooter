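; Ammo component that tracks an actor's clip and reserve ammo, starting both full at BeginPlay.
; UpdateAmmo applies a clamped change to the clip, sets CanFire while rounds remain, and prints a debug count.
; Reload works only when CanFire is false, using a timer to refill the clip from the reserve after TimeLoad.
; AddAmmoAmount accepts only non-negative pickups, capped at the default reserve; getters expose reserve, clip count and fill ratio.
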(event `self.ReceiveBeginPlay`
  (set `self.AmmoAmount` (`self.AmmoAmuntDefualt`))
  (`self.UpdateAmmo` (`self.ClipSize`)))

(event `Reload`
  (if (not (`self.CanFire`))
    (`KismetSystemLibrary.K2_SetTimerDelegate` (delegate `ReloadEnd`) (`self.TimeLoad`))))

(event `ReloadEnd`
  (`self.UpdateAmmoAmountLeft`))

(fn `AddAmmoAmount`
  (params (Delta :type Integer))
  (if (>= Delta 0)
    (set `self.AmmoAmount` (`KismetMathLibrary.Clamp` (+ Delta (`self.AmmoAmount`)) 0 (`self.AmmoAmuntDefualt`)))
    (else
      (`KismetSystemLibrary.PrintString` "No se sumó valor negativo  a la cantidad totoal de ammo"))))

(fn `GetAmmo`
  (returns (Ammo :type Integer) (AmmoByone :type "Float (double-precision)"))
  (bind _ammo (`self.Ammo`))
  (return _ammo (/ (`KismetMathLibrary.Conv_IntToDouble` _ammo) (`KismetMathLibrary.Conv_IntToDouble` (`self.ClipSize`)))))

(fn `GetAmmoAmmount`
  (returns (AmmoAmount :type Integer))
  (return (`self.AmmoAmount`)))

(fn `UpdateAmmo`
  (params (Delta :type Integer))
  (bind _output_get (set `self.Ammo` (`KismetMathLibrary.Clamp` (+ Delta (`self.Ammo`)) 0 (`self.ClipSize`))))
  (`KismetSystemLibrary.PrintString` (`KismetStringLibrary.Concat_StrStr` (`KismetSystemLibrary.GetDisplayName` (`self.GetOwner`)) "  left: " (`KismetStringLibrary.Conv_DoubleToString` (`KismetMathLibrary.Conv_IntToDouble` _output_get)) "  In Ammo component") true true (struct :`R` 1.0 :`G` 0.594703 :`B` 0.101584 :`A` 1.0)) ; For debugging
  (if (> _output_get 0)
    (set `self.CanFire` true)
    (else
      (set `self.CanFire` false))))

(fn `UpdateAmmoAmountLeft`
  (if (>= (`self.AmmoAmount`) (`self.ClipSize`))
    (`self.UpdateAmmo` (`self.ClipSize`))
    (set `self.AmmoAmount` (`KismetMathLibrary.Clamp` (- (`self.AmmoAmount`) (`self.ClipSize`)) 0 (`self.AmmoAmuntDefualt`)))
    (else
      (`self.UpdateAmmo` (`self.AmmoAmount`))
      (set `self.AmmoAmount` 0))))
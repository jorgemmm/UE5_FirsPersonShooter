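; Game state for an FPS round in which the player must destroy all drones before time runs out.
; On BeginPlay it disables player input and reads the time limit, drone count and start delay from FPSGameMode.
; A looping timer drives a session-state machine, counting down Warmup before enabling input, then the In Progress time limit.
; DroneDied handles player death and drone kills; win, death or timeout disables input and stops the timer.
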(event `self.ReceiveBeginPlay`
  (`|ExecutionSequence`
    (:`then_0`
      ;[1 1 1] Disable input and mouse cursor at all player controller
      (`self.CheckEnableInputs` false))
    (:`then_1`
      ;[1 1 1] Set Initial Value in Session state enum,  Set How to change the state over the game
      (set `self.SessionState` "NewEnumerator0"))
    (:`then_2`
      ;[1 1 1] Get Values to determine how to game and how to win form GameMode
      (bind _asfpsgame_mode (cast `/Game/Blueprints/GameModes/FPSGameMode` (`GameplayStatics.GetGameMode`)))
      (set `self.TimeLimitToClear` (`/Game/Blueprints/GameModes/FPSGameMode.GetTimeToClear` _asfpsgame_mode))
      (set `self.NumOfDrones` (`/Game/Blueprints/GameModes/FPSGameMode.GetRemainingDrones` _asfpsgame_mode))
      (bind _delaytostart (`/Game/Blueprints/GameModes/FPSGameMode.GetDelayToStart` _asfpsgame_mode))
      (set `self.DelayToSart` _delaytostart)
      (set `self.Count` _delaytostart))
    (:`then_3`
      (`KismetSystemLibrary.K2_SetTimer` null "CheckSessionState" (`self.Time`) true))))

(event `CheckSessionState`
  (switch `/Game/Blueprints/GameModes/SessionState_E` (`self.SessionState`)
    (:`NewEnumerator0`
      (`self.UpdateTimeDelayToStart`))
    (:`NewEnumerator1`
      (`self.UpdateTimeRemainig`))
    (:`NewEnumerator2`
      (`KismetSystemLibrary.K2_ClearTimer` null "CheckSessionState" :!label _label))
    (:`NewEnumerator3`
      (goto _label))
    (:`NewEnumerator4`
      (goto _label))))

(event `self.ReceiveTick`
  (params (DeltaSeconds :type "Float (single-precision)"))
  ;[1 0.008567 0.02293] Debugging
)

(fn `ChangeState`
  (params (NewSessionState :type "/Game/Blueprints/GameModes/SessionState_E Enum" :default "NewEnumerator0"))
  (set `self.SessionState` NewSessionState))

(fn `CheckEnableInputs`
  (params (NewState :type Boolean))
  (for _array_element (`self.PlayerArray`)
    (bind _asfpsplayer_controller (cast `/Game/Blueprints/PlayerState/FPSPlayerController` (`PlayerState.GetPlayerController` _array_element)))
    (`/Game/Blueprints/PlayerState/FPSPlayerController.SetPlayerEnablestate` _asfpsplayer_controller NewState)))

(fn `Drone Died`
  (params (Player :type "/Game/Blueprints/Character/FPS_Character Object Reference"))
  (`/Engine/EditorBlueprintResources/StandardMacros.IsValid` Player
    (:`Is Valid`
      (if (`/Game/Blueprints/Character/FPS_Character.GetIsDead` Player)
        (set `self.SessionState` "NewEnumerator3")
        (`KismetSystemLibrary.K2_ClearTimer` null "CheckSessionState" :!label _label)
        (`self.CheckEnableInputs` false)
        (else
          (bind _result (`/Engine/EditorBlueprintResources/StandardMacros.DecrementInt` (`self.NumOfDrones`) :!label _label_2)
            (:`  `
              (if (<= _result 0)
                (set `self.SessionState` "NewEnumerator4")
                (goto _label)
                (else
                  (set `self.SessionState` "NewEnumerator1"))))))))
    (:`Is Not Valid`
      (if (`|EnumEquality` (`self.SessionState`) "NewEnumerator1")
        (goto _label_2)))))

(fn `Get Warmup Time`
  (returns (WarmupTime :type "Float (double-precision)"))
  (return (`self.WarmupTime`)))

(fn `GetCount`
  (returns (Count :type Integer))
  (return (`self.Count`)))

(fn `GetNumberOfDrones`
  (returns (NumOfDrones :type Integer))
  (return (`self.NumOfDrones`)))

(fn `getSessionState`
  (returns (SessionState :type "/Game/Blueprints/GameModes/SessionState_E Enum"))
  (return (`self.SessionState`)))

(fn `GetTimeRemaining`
  (returns (TimeLimitToClear :type Integer))
  (return (`self.TimeLimitToClear`)))

(fn `NewFunction_0`)

(fn `UpdateTimeDelayToStart`
  (bind _output_get (set `self.Count` (`KismetMathLibrary.Clamp` (- (`self.Count`) 1) 0 (`self.DelayToSart`))))
  (if (<= _output_get 0)
    (`self.ChangeState` "NewEnumerator1")
    (`self.CheckEnableInputs` true)))

(fn `UpdateTimeRemainig`
  (if (`|EnumEquality` (`self.SessionState`) "NewEnumerator1")
    (bind _output_get (set `self.TimeLimitToClear` (`KismetMathLibrary.Clamp` (- (`self.TimeLimitToClear`) (`KismetMathLibrary.Conv_Int64ToInt` (`KismetMathLibrary.FTrunc64` (`self.Time`)))) 0 300)))
    (if (<= _output_get 0)
      (set `self.SessionState` "NewEnumerator2")
      (`self.CheckEnableInputs` false)
      (else
        (set `self.SessionState` "NewEnumerator1")))))

(fn `UserConstructionScript`)
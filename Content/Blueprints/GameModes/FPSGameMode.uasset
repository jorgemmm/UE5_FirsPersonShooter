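; FPS game mode that tracks a drone-clearing objective and decides when the player wins or loses.
; BeginPlay gathers all DronePawn actors once through a costly world search, stores their count and caches the player character as Hero.
; DroneDied treats Hero's death as a loss, otherwise decrements the count until a win; outcomes only print strings.
; Getters expose remaining drones, clear time and start delay; HUD creation is disconnected.
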(event `self.ReceiveBeginPlay`
  (`|ExecutionSequence`
    (:`then_1`
      ;[1 1 1] Get drones over map an number of drones
      (bind _output_get (set `self.Drones` (`self.GetDrones`)))
      (set `self.NumberOfDrones` (`KismetArrayLibrary.Array_Length` _output_get)))
    (:`then_2`
      ;[1 1 1] Reference player
      (set `self.Hero` (cast `/Game/Blueprints/Character/FPS_Character` (`GameplayStatics.GetPlayerPawn` 0) :!pure true)))))

(fn `DroneDied`
  (params (ActorDied :type "Actor Object Reference"))
  ;[0.1343 0.1343 0.1343] Es mejor esta lógica en game estate
  (if (== ActorDied (`self.Hero`))
    (`KismetSystemLibrary.PrintString` "Call Game over - Lose")
    (else
      (bind _result (`/Engine/EditorBlueprintResources/StandardMacros.DecrementInt` (`self.NumberOfDrones`))
        (:`  `
          (if (<= _result 0)
            (`KismetSystemLibrary.PrintString` "Call Game over - Win")
            (else
              (`KismetSystemLibrary.PrintString` "conitinue  Game kill drone left"))))))))

(fn `GetDelayToStart`
  (returns (DelayToStart :type Integer))
  (return (`self.DelayToStart`)))

(fn `GetDrones`
  (returns (Output_Get :type "Array of /Game/Blueprints/Drone/DronePawn Object Reference"))
  ;[1 1 1] No llamar esta función mucho, alto coste computacinal
  (bind _outactors (`GameplayStatics.GetAllActorsOfClass` "/Game/Blueprints/Drone/DronePawn.DronePawn_C"))
  (return _outactors))

(fn `GetRemainingDrones`
  (returns (RemainingDrones :type Integer))
  (return (`self.NumberOfDrones`)))

(fn `GetTimeToClear`
  (returns (TimeToClearZome :type Integer))
  (return (`self.TimeToClearZome`)))

(fn `UserConstructionScript`)